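; A gravity plate actor, apparently meant to redirect the player's gravity along a chosen horizontal direction, but left unfinished.
; Tick casts and caches the player character and checks Enabled, with nothing wired after the check.
; Disconnected nodes map Direction to a Gravity vector, with capsule and actor rotation only for Left.
; A separate, also disconnected node would pass that vector to the player's gravity movement component.
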(event EventBeginPlay)

(event Collision|EventActorBeginOverlap
  (params (OtherActor :type Actor%20Object%20Reference)))

(event EventTick
  (params (DeltaSeconds :type Float%20%28single-precision%29))
  (bind _asplayer_character (Utilities|Casting|CastToPlayerCharacter (Game|Player|GetPlayerPawn 0)))
  (Variables|Default|SetAs%20Player%20Character _asplayer_character)
  (if (Variables|Default|GetEnabled)
    _))

(fn ConstructionScript)