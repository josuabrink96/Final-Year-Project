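; Player character Blueprint that handles basic input state for the player.
; On BeginPlay it sets game-only input mode, and the W key sets a Moving flag while held.
; A disconnected pause-menu chain would create and cache a widget, show the cursor, switch to UI-only input and pause the game, but nothing triggers it.
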(event EventBeginPlay
  (Input|SetInputModeGameOnly (Game|GetPlayerController 0)))

(event Input|KeyboardEvents|W
  (params (Key :type Key%20Structure :default "None"))
  (:Pressed
    (Variables|Default|SetMoving true))
  (:Released
    (Variables|Default|SetMoving false)))

(fn ConstructionScript)